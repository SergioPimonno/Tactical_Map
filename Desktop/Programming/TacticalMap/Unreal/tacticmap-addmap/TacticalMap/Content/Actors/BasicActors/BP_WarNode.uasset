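; BP_WarNode is an actor holding a shared Shoot function for ranged attacks.
; Shoot spawns a scaled-down BP_Projectile at the target mesh's "SocketShoot" socket, aimed at the enemy, and passes it the damage.
; A height check boosts damage when the owner stands sufficiently above the enemy.
; The reduced-damage branch has an unconnected validity check, so its penalty does not apply.
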(event Collision|EventActorBeginOverlap
  (params (OtherActor :type Actor%20Object%20Reference)))

(event EventTick
  (params (DeltaSeconds :type Float%20%28single-precision%29)))

(fn ConstructionScript)

(fn Shoot
  (params (Owner :type BP%20Army%20Basic%20Object%20Reference) (Enemy :type BP%20Army%20Basic%20Object%20Reference) (Damage :type Float%20%28single-precision%29) (target :type Object%20Object%20Reference))
  (bind _returnvalue (Transformation|GetActorLocation Enemy))
  (bind _returnvalue_2 (Transformation|GetActorLocation Owner))
  (bind _returnvalue_3 (- (.z _returnvalue_2) (.z _returnvalue)))
  (Utilities|FlowControl|Sequence
    (:then_0
      (bind _asstatic_mesh_component (Utilities|Casting|CastToStaticMeshComponent target))
      (bind _returnvalue_4 (Game|SpawnActorfromClass "/Game/Actors/BP_Projectile.BP_Projectile_C" (Math|Transform|MakeTransform (Transformation|GetSocketLocation _asstatic_mesh_component "SocketShoot") (Math|Rotator|FindLookatRotation (Transformation|GetSocketLocation _asstatic_mesh_component "SocketShoot") (Transformation|GetActorLocation Enemy)) "0.070000,0.070000,0.070000") "Undefined" 0 0))
      (Variables|/Game/Actors/BP_Projectile.BP_Projectile_C|SetDamage _returnvalue_4 Damage))
    (:then_1
      (if (>= _returnvalue_3 5.0)
        (Utilities|IsValid _returnvalue_4
          (:Is%20Valid
            (Variables|/Game/Actors/BP_Projectile.BP_Projectile_C|SetDamage _returnvalue_4 (* Damage 1.5))))
        (elif (<= _returnvalue_3 5.0)
          (Utilities|IsValid 0
            (:Is%20Valid
              (Variables|/Game/Actors/BP_Projectile.BP_Projectile_C|SetDamage _returnvalue_4 (* Damage 0.5)))))))))