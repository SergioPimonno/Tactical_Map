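; BP_ArmyBasic is a team-based army squad that fights opposing squads through its child BP_WarNode actors, colored green or red by team.
; A bound Start event gathers other-team squads, picks a random target, then starts looping timers to face it and fire from random nodes.
; Tick checks intend health-based node removal and squad death, but read an unexecuted loop's output.
; The behavior tree call is disconnected.
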(event Custom|SercEnemy
  ;[1 1 1] Adding Enemy to Enemy Array
  (bind _outactors (Actor|GetAllActorsOfClass "BP_ArmyBasic_C"))
  (for _array_element _outactors
    (if (not (== (Variables|BP_ArmyBasic_C|GetTeam _array_element) (Variables|Param|GetTeam)))
      (Utilities|Array|Add (Variables|Default|GetEnemys) _array_element)))
  (Variables|Default|SetReadyToAtack true)
  (CallFunction|Attack))

(event Custom|Attack
  (CallFunction|GetEnemy)
  (Utilities|Time|SetTimerbyEvent (delegate Custom|Position) 1.0 true)
  (Utilities|Time|SetTimerbyEvent (delegate Custom|Shoot) (Variables|Param|GetSpeedShoot) true))

(event Custom|Death
  ;[1 1 1] Death
  (EventDispatchers|UnbindEventfromStart (delegate Custom|SercEnemy))
  (Actor|DestroyActor))

(event Custom|Position
  ;[1 1 1] Targeting to Enemy
  (if (Variables|Default|GetReadyToAtack)
    (Utilities|IsValid (Variables|Default|GetEnemy)
      (:Is%20Valid
        (Transformation|SetRelativeRotation (Variables|Transformation|GetRootComponent) (Math|Rotator|MakeRotator 0.0 0.0 (.yaw (Math|Rotator|FindLookatRotation (Transformation|GetActorLocation) (Transformation|GetActorLocation (Variables|Default|GetEnemy))))) false false))
      (:Is%20Not%20Valid
        (Variables|Default|SetReadyToAtack false)
        (Utilities|Array|RemoveItem (Variables|Default|GetEnemys) (Variables|Default|GetEnemy))
        (CallFunction|SercEnemy)))))

(event Custom|Shoot
  (bind _controlledactors (Variables|Default|GetControlledActors))
  ;[1 1 1] Shooting
  (if (Variables|Default|GetReadyToAtack)
    (bind _asbp_war_node (Utilities|Casting|CastToBP_WarNode (Utilities|Array|Get(acopy) _controlledactors (Math|Random|RandomInteger (Utilities|Array|Length _controlledactors)))))
    (Default|Shoot _asbp_war_node self (Variables|Default|GetEnemy) (Variables|Param|GetDamage) (Variables|/Game/Actors/BasicActors/BP_WarNode.BP_WarNode_C|GetStaticMesh _asbp_war_node))))

(event Collision|EventActorBeginOverlap
  (params (OtherActor :type Actor%20Object%20Reference)))

(event EventTick
  (params (DeltaSeconds :type Float%20%28single-precision%29))
  (bind _controlledactors (Variables|Default|GetControlledActors))
  (Utilities|FlowControl|Sequence
    (:then_0
      (if (<= (stale _array_element) (Variables|Default|GetDeathHealth))
        (bind _output_get (Variables|Default|SetChildActorDestroy (Utilities|Array|Get(acopy) _controlledactors (Math|Random|RandomInteger (Utilities|Array|Length _controlledactors)))))
        (Utilities|IsValid _output_get
          (:Is%20Valid
            (Actor|DestroyActor _output_get)
            (Utilities|Array|RemoveItem _controlledactors _output_get)
            (Variables|Default|SetDeathHealth (Variables|Default|GetDeathHealth)))
          (:Is%20Not%20Valid
            (CallFunction|Death)))))
    (:then_1
      (if (<= (stale _array_element) 0.0)
        (CallFunction|Death)))
    (:then_2
      (if (== (Utilities|Array|Length (Variables|Default|GetEnemys)) 0)
        (Variables|Default|SetReadyToAtack false)))))

(event EventBeginPlay
  (bind _childactors (Actor|GetAllChildActors true))
  (Utilities|FlowControl|Sequence
    (:then_0
      ;[1 1 1] Setting up Unit HP
      (bind _output_get (Variables|Param|SetHealthSol 2e+01))
      (bind _output_get_2 (Variables|Param|SetHeathBTR 5e+01))
      (bind _output_get_3 (Variables|Param|SetHealthTank 1e+02)))
    (:then_2
      (Variables|Default|SetSpawnCollisionHandlingMethod "AdjustIfPossibleButDontSpawnIfColliding")
      (EventDispatchers|BindEventtoStart (delegate Custom|SercEnemy))
      (Variables|Default|SetControlledActors _childactors)
      ;[1 1 1] Team Setting
      (for _array_element _childactors
        (switch int (Variables|Param|GetTeam)
          (:0
            (bind _asbp_war_node (Utilities|Casting|CastToBP_WarNode _array_element))
            (Rendering|Material|SetMaterial (Variables|/Game/Actors/BasicActors/BP_WarNode.BP_WarNode_C|GetStaticMesh _asbp_war_node) 0 "/AnimationSharing/AnimSharingGreen.AnimSharingGreen"))
          (:1
            (bind _asbp_war_node_2 (Utilities|Casting|CastToBP_WarNode _array_element))
            (Rendering|Material|SetMaterial (Variables|/Game/Actors/BasicActors/BP_WarNode.BP_WarNode_C|GetStaticMesh _asbp_war_node_2) 0 "/AnimationSharing/AnimSharingRed.AnimSharingRed")))))))

(fn ConstructionScript)

(fn GetEnemy
  (bind _enemys (Variables|Default|GetEnemys))
  (Variables|Default|SetEnemy (Utilities|Array|Get(acopy) _enemys (Math|Random|RandomInteger (Utilities|Array|Length _enemys)))))